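; BP_BaseCharacter is a character Blueprint that shows network role and player name through an overhead widget.
; On BeginPlay it casts OverHeadWidget's user widget to WBP_OverheadWidget, waits briefly, then calls ShowPlayerNetRole with itself and the PlayerState name.
; It passes "default" as the name if the PlayerState is still invalid after that single delay.
; Tick, overlap and construction logic are empty.
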(event `self.ReceiveBeginPlay`
  (bind _aswbp_overhead_widget (cast `/Game/MainFolder/HUD/WBP_OverheadWidget` (`WidgetComponent.GetUserWidgetObject` (`self.OverHeadWidget`))))
  (`KismetSystemLibrary.Delay` 0.2)
  (`/Engine/EditorBlueprintResources/StandardMacros.IsValid` (`GameplayStatics.GetPlayerState` 0)
    (:`Is Valid`
      (`OverHeadWidget.ShowPlayerNetRole` _aswbp_overhead_widget self (`PlayerState.GetPlayerName` (`GameplayStatics.GetPlayerState` 0))))
    (:`Is Not Valid`
      (`OverHeadWidget.ShowPlayerNetRole` _aswbp_overhead_widget self "default"))))

(fn `UserConstructionScript`)